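; Prototype actor that builds a unit cube as a procedural mesh, apparently a first step toward a cube sphere.
; GenerateMesh runs on construction and BeginPlay, creating eight shared corner vertices and six quads of two triangles each.
; SplitQuad is unfinished: for quad 0 it appends the diagonal midpoint as a vertex, collects unique indices and prints debug output, but never rebuilds the triangles.
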(event EventBeginPlay
  (CallFunction|GenerateMesh))

(event Collision|EventActorBeginOverlap
  (params (OtherActor :type Actor%20Object%20Reference)))

(event EventTick
  (params (DeltaSeconds :type Float%20%28single-precision%29)))

(fn ConstructionScript
  (CallFunction|GenerateMesh))

(fn GenerateMesh
  (CallFunction|CreateVertices (LocalVariables|GetVertices))
  (CallFunction|CreateTriangles (LocalVariables|GetTriangles))
  (CallFunction|SplitQuad (LocalVariables|GetTriangles) (LocalVariables|GetVertices))
  (Class|ProceduralMeshComponent|CreateMeshSectionLinearColor (Variables|Default|GetProceduralMesh) 0 (LocalVariables|GetVertices) (LocalVariables|GetTriangles) 0 0 0 0 0 0 0 false))

(fn CreateVertices
  (params (Vertices :type Array%20of%20Vectors))
  (Utilities|FlowControl|Sequence
    (:then_0
      (Utilities|Array|Add Vertices "1.000000,1.000000,0.000000")
      (Utilities|Array|Add Vertices "1.000000,0.000000,0.000000")
      (Utilities|Array|Add :TargetArray Vertices)
      (Utilities|Array|Add Vertices "0.000000,1.000000,0.000000"))
    (:then_1
      (Utilities|Array|Add Vertices "1.000000,1.000000,1.000000")
      (Utilities|Array|Add Vertices "1.000000,0.000000,1.000000")
      (Utilities|Array|Add Vertices "0.000000,0.000000,1.000000")
      (Utilities|Array|Add Vertices "0.000000,1.000000,1.000000"))
    (:then_2
      (return))))

(fn CreateTriangles
  (params (Triangles :type Array%20of%20Integers))
  (Utilities|FlowControl|Sequence
    (:then_0
      (bind _triangles (CallFunction|CreateQuadTriangles 3 2 1))
      (Utilities|Array|AppendArray Triangles _triangles))
    (:then_1
      (bind _triangles_2 (CallFunction|CreateQuadTriangles 4 5 6 7))
      (Utilities|Array|AppendArray Triangles _triangles_2))
    (:then_2
      (bind _triangles_3 (CallFunction|CreateQuadTriangles 0 1 5 4))
      (Utilities|Array|AppendArray Triangles _triangles_3))
    (:then_3
      (bind _triangles_4 (CallFunction|CreateQuadTriangles 4 7 3))
      (Utilities|Array|AppendArray Triangles _triangles_4))
    (:then_4
      (bind _triangles_5 (CallFunction|CreateQuadTriangles 1 2 6 5))
      (Utilities|Array|AppendArray Triangles _triangles_5))
    (:then_5
      (bind _triangles_6 (CallFunction|CreateQuadTriangles 2 3 7 6))
      (Utilities|Array|AppendArray Triangles _triangles_6))
    (:then_6
      (return))))

(fn CreateQuadTriangles
  (params (Vertex0 :type Integer) (Vertex1 :type Integer) (Vertex2 :type Integer) (Vertex3 :type Integer))
  (return (Utilities|Array|MakeArray Vertex0 Vertex1 Vertex2 Vertex2 Vertex3 Vertex0)))

(fn GetQuadsCount
  (params (Triangles :type Array%20of%20Integers))
  (return (/ (Utilities|Array|Length Triangles) (Variables|Default|GetCountOfIndexesCreatingQuad))))

(fn SplitQuad
  (params (Triangles :type Array%20of%20Integers) (Vertices :type Array%20of%20Vectors) (QuadIndex :type Integer))
  (bind _quadindexbuffer (LocalVariables|GetQuadIndexBuffer))
  (bind _countofindexescreatingquad (Variables|Default|GetCountOfIndexesCreatingQuad))
  (bind _returnvalue (* QuadIndex _countofindexescreatingquad))
  (bind _output (Utilities|Array|Get(acopy) _quadindexbuffer))
  (bind _output_2 (Utilities|Array|Get(acopy) _quadindexbuffer 2))
  (bind _output_3 (Utilities|Array|Get(acopy) Vertices _output_2))
  (bind _output_4 (Utilities|Array|Get(acopy) Vertices _output))
  (bind _middlepoint (CallFunction|GetMiddlePoint _output_4 _output_3))
  ;[1 1 1] Validate Quad Index
  (Math|Integer|CompareInt QuadIndex (CallFunction|GetQuadsCount Triangles)
    (:>
      (Development|PrintString "Invalid Quad Index" false true "(R=1.000000,G=0.000000,B=0.000000,A=1.000000)" :!label _label)
      (return))
    (:==
      (goto _label))
    (:<
      (Development|PrintString "Split quad")
      ;[1 1 1] Get first and last index of quad index buffer
      (LocalVariables|SetQuadFirtIndex _returnvalue)
      (LocalVariables|SetQuadLastIndex (+ _returnvalue (Variables|Default|GetCountOfIndexesCreatingQuad) -1))
      (for _index (range (LocalVariables|GetQuadFirtIndex) (LocalVariables|GetQuadLastIndex)) ; Iterate over index buffer of quad
        ;[1 1 1] Gather index buffer of quad
        (Utilities|Array|Add (LocalVariables|GetQuadIndexBuffer) (Utilities|Array|Get(acopy) Triangles _index))
        (Development|PrintString (Utilities|String|Append "Triangle index: " (Utilities|String|ToString(Integer) _index) " Value: " (Utilities|String|ToString(Integer) (Utilities|Array|Get(acopy) Triangles _index))) false true "(R=1.000000,G=0.000000,B=0.000000,A=1.000000)"))
      (Utilities|FlowControl|Sequence
        (:then_0
          ;[1 1 1] Get middle point of Quad "The split point"
          (LocalVariables|SetMiddlePoint _middlepoint)
          (Development|PrintString (Utilities|String|Append "Middle point: " (Utilities|String|ToString(Vector) _middlepoint))))
        (:then_1
          ;[1 1 1] Add middle point to vertices and save his index
          (bind _returnvalue_2 (Utilities|Array|Add Vertices (LocalVariables|GetMiddlePoint)))
          (LocalVariables|SetMiddlePointIndex _returnvalue_2))
        (:then_2
          ;[1 1 1] Get all unique indexes
          (for _array_element (LocalVariables|GetQuadIndexBuffer)
            (Utilities|Array|AddUnique (LocalVariables|GetQuadUniqueIndexes) _array_element)))
        (:then_3
          (Development|PrintString "Quad unique indexes")
          (for _array_element_2 (LocalVariables|GetQuadUniqueIndexes)
            (Development|PrintString (Utilities|String|ToString(Integer) _array_element_2))))))))

(fn GetMiddlePoint
  (params (FirstPoint :type Vector) (SecondPoint :type Vector))
  (return (/ (+ FirstPoint SecondPoint) 2.0)))