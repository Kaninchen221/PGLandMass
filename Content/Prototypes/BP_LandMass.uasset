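; Prototype landmass actor that builds a procedural mesh at BeginPlay from a small vertex grid with a vertex-color material.
; Unconnected ApplyHeight is written to displace vertex Z by summing Perlin noise octaves, scaled by lacunarity and persistence.
; CreateColors maps height bands to grey, green or blue but is never called, so the mesh gets neither noise height nor those colors.
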(event EventBeginPlay
  (CallFunction|CreateMesh))

(event Collision|EventActorBeginOverlap
  (params (OtherActor :type Actor%20Object%20Reference)))

(event EventTick
  (params (DeltaSeconds :type Float%20%28single-precision%29)))

(fn ConstructionScript)

(fn CreateMesh
  (Class|PGLandMass|CreateVertices (Utilities|Struct|MakeIntPoint 4 4) "(X=1.500000,Y=1.500000)")
  (Class|PGLandMass|CreateTriangles)
  (Class|ProceduralMeshComponent|CreateMeshSectionLinearColor (Variables|Default|GetMeshComponent) 0 (Variables|Default|GetVertices) (Variables|Default|GetTriangles) 0 0 0 0 0 0 0 false)
  (Rendering|Material|SetMaterial (Variables|Default|GetMeshComponent) 0 "/PGSpherePlugin/Prototypes/M_VertexColor.M_VertexColor"))

(fn ApplyHeight
  (Class|PGPerlinNoise|Reseed (Variables|Default|GetPerlinNoise) (.Milliseconds (Math|Timespan|BreakTimespan (TimeOfDay|GetTimeOfDay (Math|DateTime|MakeDateTime 2021 2 2 1 1 1 1) :!class /Script/Engine.KismetMathLibrary))))
  (for _index (range 0 (- (Utilities|Array|Length (Variables|Default|GetVertices)) 1))
    (LocalVariables|SetVertexIndex _index)
    (LocalVariables|SetVertex (Utilities|Array|Get(acopy) (Variables|Default|GetVertices) (LocalVariables|GetVertexIndex)))
    (Utilities|FlowControl|Sequence
      (:then_0
        (for _index_2 (range 0 (LocalVariables|GetOctavesCount))
          (bind _value (CallFunction|Random 2.0 0.5 (Math|Conversions|ToFloat(Integer) _index_2) (.x (LocalVariables|GetVertex)) (.y (LocalVariables|GetVertex))))
          (Utilities|Array|Add (LocalVariables|GetOctavesValue) _value)))
      (:then_1
        (for _array_element (LocalVariables|GetOctavesValue)
          (LocalVariables|SetZValue (+ _array_element (LocalVariables|GetZValue))))
        (Class|KismetMathLibrary|VectorSet (Utilities|Array|Get(acopy) (Variables|Default|GetVertices) (LocalVariables|GetVertexIndex)) (.x (LocalVariables|GetVertex)) (.y (LocalVariables|GetVertex)) (/ (LocalVariables|GetZValue) 3.0))
        (LocalVariables|SetZValue 0.0)))))

(fn Random
  (params (Lacunarity :type Float%20%28single-precision%29) (Persistance :type Float%20%28single-precision%29) (Octave :type Float%20%28single-precision%29) (X :type Float%20%28single-precision%29) (Y :type Float%20%28single-precision%29))
  (LocalVariables|SetFrequency (|(pow(Lacunarity,Octave)) Lacunarity Octave)) ; Calculate Frequency
  (LocalVariables|SetAmplitude (|(pow(Persistance,Octave)) Persistance Octave)) ; Calculate Amplitude
  (return (* (Class|PGPerlinNoise|NormalizedOctaveNoise3D (Variables|Default|GetPerlinNoise) (+ (* X (LocalVariables|GetFrequency)) 0.1) (+ 0.1 (* (LocalVariables|GetFrequency) Y)) (+ (Math|Conversions|ToFloat(Integer) (.Millisecond (Math|DateTime|BreakDateTime (Math|DateTime|Now)))) 0.1) (Math|Float|Truncate (+ Octave 1.0))) (LocalVariables|GetAmplitude))))

(fn CreateColors
  (params (Vertices :type Array%20of%20Vectors))
  (for _array_element Vertices
    (Math|Float|CompareFloat (.Z (Math|Vector|BreakVector _array_element)) 0.7
      (:>
        (Utilities|Array|Add (LocalVariables|GetColors) "(R=0.221618,G=0.229167,B=0.226847,A=1.000000)" :!label _label))
      (:==
        (goto _label))
      (:<
        (Math|Float|CompareFloat (.Z (Math|Vector|BreakVector _array_element)) -0.3
          (:>
            (Utilities|Array|Add (LocalVariables|GetColors) "(R=0.156161,G=0.333333,B=0.065612,A=1.000000)" :!label _label_2))
          (:==
            (goto _label_2))
          (:<
            (Utilities|Array|Add (LocalVariables|GetColors) "(R=0.097912,G=0.126194,B=0.333333,A=1.000000)"))))))
  (return (LocalVariables|GetColors)))