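; Prototype procedural sphere actor that currently builds only a six-vertex, eight-triangle octahedron, with no subdivision.
; CreateMesh runs from both the construction script and BeginPlay, filling a ProceduralMesh section and applying a debug material.
; Helper functions supply hardcoded vertices, triangle indices, white vertex colors and a repeating placeholder UV pattern.
; Normals and tangents come from CalculateTangentsForMesh, leaving the CreateTangets function as an empty stub.
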(event EventBeginPlay
  (CallFunction|CreateMesh))

(event Collision|EventActorBeginOverlap
  (params (OtherActor :type Actor%20Object%20Reference)))

(event EventTick
  (params (DeltaSeconds :type Float%20%28single-precision%29)))

(fn ConstructionScript
  (CallFunction|CreateMesh))

(fn CreateMesh
  (bind _vertices (CallFunction|CreateVertices))
  (bind _output_get (LocalVariables|SetVerticies _vertices))
  (LocalVariables|SetVerticesCount (Utilities|Array|Length _output_get))
  (bind _specifiedtriangles (CallFunction|CreateTriangles))
  (LocalVariables|SetTriangles _specifiedtriangles)
  (bind _vertexcolors (CallFunction|CreateVertexColors))
  (LocalVariables|SetVertexColors _vertexcolors)
  (bind _uv (CallFunction|CreateUV (LocalVariables|GetVerticesCount)))
  (LocalVariables|SetUV _uv)
  (bind (_normals _tangents) (Class|KismetProceduralMeshLibrary|CalculateTangentsforMesh (LocalVariables|GetVerticies) (LocalVariables|GetTriangles) (LocalVariables|GetUV)))
  (LocalVariables|SetNormals _normals)
  (LocalVariables|SetTangets _tangents)
  (Class|ProceduralMeshComponent|CreateMeshSectionLinearColor (Variables|Default|GetProceduralMesh) 0 (LocalVariables|GetVerticies) (LocalVariables|GetTriangles) (LocalVariables|GetNormals) (LocalVariables|GetUV) 0 0 0 (LocalVariables|GetVertexColors) (LocalVariables|GetTangets) false)
  (Rendering|Material|SetMaterial (Variables|Default|GetProceduralMesh) 0 "/PGSpherePlugin/Prototypes/M_SphereDebug.M_SphereDebug"))

(fn CreateVertices
  (return (Utilities|Array|MakeArray (Math|Vector|MakeVector 0.0 0.0 0.0) (Math|Vector|MakeVector 1.0 0.0 0.0) (Math|Vector|MakeVector 0.0 1.0 0.0) (Math|Vector|MakeVector 1.0 1.0 0.0) (Math|Vector|MakeVector 0.5 0.5 0.707107) (Math|Vector|MakeVector 0.5 0.5 -0.707107))))

(fn CreateTriangles
  (bind _output_get (LocalVariables|SetTriangles (Utilities|Array|MakeArray 0 4 1 1 4 3 3 4 2 2 4 0)))
  (Utilities|Array|AppendArray _output_get (Utilities|Array|MakeArray 5 0 1 5 1 3 5 3 2 5 2 0))
  (return (LocalVariables|GetTriangles)))

(fn CreateVertexColors
  (bind _linearcolor (Utilities|Struct|MakeLinearColor 1.0 1.0 1.0 1.0))
  (return (Utilities|Array|MakeArray _linearcolor _linearcolor _linearcolor _linearcolor _linearcolor _linearcolor)))

(fn CreateUV
  (params (VerticesCount :type Integer))
  (for _index (range 1 (/ VerticesCount 3))
    (Utilities|Array|AppendArray (LocalVariables|GetUVs) (Utilities|Array|MakeArray "(X=0.000000,Y=0.000000)" "(X=0.000000,Y=1.000000)" "(X=1.000000,Y=0.000000)")))
  (return (LocalVariables|GetUVs)))

(fn CreateTangets)