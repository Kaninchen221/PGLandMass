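; Prototype actor that, despite its sphere name, builds a flat triangulated procedural mesh with a debug material, on construction and BeginPlay.
; CreateVertices lays out staggered XY rows alternating between Rows and Rows-1 points.
; CreateTriangles links neighboring rows in forward and backward passes, using FlipFlops for row parity and helpers for flat vertex indices.
; Placeholder UVs and white vertex colors join calculated normals and tangents in one mesh section.
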(event EventBeginPlay
  (CallFunction|CreateMesh))

(event Collision|EventActorBeginOverlap
  (params (OtherActor :type Actor%20Object%20Reference)))

(event EventTick
  (params (DeltaSeconds :type Float%20%28single-precision%29)))

(fn ConstructionScript
  (CallFunction|CreateMesh))

(fn CreateMesh
  (bind _outvertices (CallFunction|CreateVertices 1.0 (LocalVariables|GetRows) "0, 0, 0"))
  (bind _output_get (LocalVariables|SetVertices _outvertices))
  (bind _output_get_2 (LocalVariables|SetVertexCount (Utilities|Array|Length _output_get)))
  (bind _outtriangles (CallFunction|CreateTriangles _output_get_2 (LocalVariables|GetRows)))
  (LocalVariables|SetTriangles _outtriangles)
  (bind _outvertexcolors (CallFunction|CreateVertexColors (LocalVariables|GetVertexCount)))
  (LocalVariables|SetVertexColors _outvertexcolors)
  (bind _outuv (CallFunction|CreateUV (LocalVariables|GetVertexCount)))
  (LocalVariables|SetUV _outuv)
  (bind (_normals _tangents) (Class|KismetProceduralMeshLibrary|CalculateTangentsforMesh (LocalVariables|GetVertices) (LocalVariables|GetTriangles) (LocalVariables|GetUV)))
  (LocalVariables|SetNormals _normals)
  (LocalVariables|SetTangets _tangents)
  (Class|ProceduralMeshComponent|CreateMeshSectionLinearColor (Variables|Default|GetProceduralMesh) 0 (LocalVariables|GetVertices) (LocalVariables|GetTriangles) (LocalVariables|GetNormals) (LocalVariables|GetUV) 0 0 0 (LocalVariables|GetVertexColors) (LocalVariables|GetTangets) false)
  (Rendering|Material|SetMaterial (Variables|Default|GetProceduralMesh) 0 "/PGSpherePlugin/Prototypes/M_SphereDebug.M_SphereDebug"))

(fn CreateVertices
  (params (Radius :type Float%20%28single-precision%29) (Rows :type Integer) (StartPoint :type Vector))
  (LocalVariables|SetPointsInRow Rows)
  (for _index (range 1 (- (* Rows 2) 1)) ; Rows
    (Utilities|FlowControl|FlipFlop
      (:A
        (for _index_2 (range 0 (- (LocalVariables|GetPointsInRow) 1))
          (Utilities|Array|Add (LocalVariables|GetVertices) (LocalVariables|GetCurrentPoint))
          (LocalVariables|SetCurrentPoint (+ (LocalVariables|GetCurrentPoint) "2.000000, 0, 0")))
        (LocalVariables|SetCurrentPoint (Math|Vector|MakeVector (+ (.x StartPoint) 1.0) (+ (.y (LocalVariables|GetCurrentPoint)) 1.0) (.z (LocalVariables|GetCurrentPoint)))))
      (:B
        (for _index_3 (range 0 (- (LocalVariables|GetPointsInRow) 2))
          (Utilities|Array|Add (LocalVariables|GetVertices) (LocalVariables|GetCurrentPoint))
          (LocalVariables|SetCurrentPoint (+ (LocalVariables|GetCurrentPoint) "2.000000, 0, 0")))
        (LocalVariables|SetCurrentPoint (Math|Vector|MakeVector (.x StartPoint) (+ (.y (LocalVariables|GetCurrentPoint)) 1.0) (.z (LocalVariables|GetCurrentPoint)))))))
  (return (LocalVariables|GetVertices)))

(fn CreateTriangles
  (params (VertexCount :type Integer) (Rows :type Integer))
  (LocalVariables|SetTotalRows (- (* Rows 2) 1))
  (Utilities|FlowControl|Sequence
    (:then_0
      ;[1 1 1] Get number of vertices for each row we will use to create middle triangles
      (bind _vertexcount (CallFunction|GetRowVertexCount 0 Rows))
      (bind _output_get (LocalVariables|SetUsedVerticesCount (- _vertexcount 1)))
      (Development|PrintString (Utilities|String|Append "Use only " (Utilities|String|ToString(Integer) _output_get) " vertices to create triangles") false))
    (:then_1
      ;[1 1 1] Iterate from 0 row to one before last
      (for _index (range 0 (- (LocalVariables|GetTotalRows) 2))
        (bind _output_get_2 (LocalVariables|SetCurrentRow _index))
        (LocalVariables|SetNextRow (+ _output_get_2 1))
        (Utilities|FlowControl|FlipFlop
          (:A
            ;[1 1 1] For even rows
            (for _index_2 (range 0 (- (LocalVariables|GetUsedVerticesCount) 1))
              (bind _output_get_3 (LocalVariables|SetCurrentVertexIndex _index_2))
              (LocalVariables|SetNextVertexIndex (+ _output_get_3 1))
              (LocalVariables|SetIndexOffset 0)
              ;[1 1 1] Create Triangle
              (Utilities|FlowControl|Sequence
                (:then_0
                  (bind _realindex (CallFunction|GetVertexRealIndex (LocalVariables|GetCurrentRow) (LocalVariables|GetCurrentVertexIndex) Rows)))
                (:then_1
                  (bind _realindex_2 (CallFunction|GetVertexRealIndex (LocalVariables|GetCurrentRow) (LocalVariables|GetNextVertexIndex) Rows)))
                (:then_2
                  (bind _realindex_3 (CallFunction|GetVertexRealIndex (LocalVariables|GetNextRow) (+ (LocalVariables|GetCurrentVertexIndex) (LocalVariables|GetIndexOffset)) Rows)))
                (:then_3
                  ;[1 1 1] Add triangle
                  (Utilities|Array|AppendArray (LocalVariables|GetTriangles) (Utilities|Array|MakeArray _realindex _realindex_2 _realindex_3))))))
          (:B
            ;[1 1 1] For not even rows
            (for _index_3 (range 0 (- (LocalVariables|GetUsedVerticesCount) 2))
              (bind _output_get_4 (LocalVariables|SetCurrentVertexIndex _index_3))
              (LocalVariables|SetNextVertexIndex (+ _output_get_4 1))
              (LocalVariables|SetIndexOffset 1)
              (Utilities|FlowControl|Sequence
                (:then_0
                  (bind _realindex_4 (CallFunction|GetVertexRealIndex (LocalVariables|GetCurrentRow) (LocalVariables|GetCurrentVertexIndex) Rows)))
                (:then_1
                  (bind _realindex_5 (CallFunction|GetVertexRealIndex (LocalVariables|GetCurrentRow) (LocalVariables|GetNextVertexIndex) Rows)))
                (:then_2
                  (bind _realindex_6 (CallFunction|GetVertexRealIndex (LocalVariables|GetNextRow) (+ (LocalVariables|GetCurrentVertexIndex) (LocalVariables|GetIndexOffset)) Rows)))
                (:then_3
                  (Utilities|Array|AppendArray (LocalVariables|GetTriangles) (Utilities|Array|MakeArray _realindex_4 _realindex_5 _realindex_6)))))))))
    (:then_2
      ;[1 1 1] Iterate from one before last row to 1
      (for _index_4 (range 1 (- (LocalVariables|GetTotalRows) 1))
        (bind _output_get_5 (LocalVariables|SetCurrentRow (- (LocalVariables|GetTotalRows) _index_4)))
        (LocalVariables|SetNextRow (- _output_get_5 1))
        (Utilities|FlowControl|FlipFlop
          (:A
            (for _index_5 (range 0 (- (LocalVariables|GetUsedVerticesCount) 1))
              (bind _output_get_6 (LocalVariables|SetCurrentVertexIndex _index_5))
              (LocalVariables|SetNextVertexIndex (+ _output_get_6 1))
              (LocalVariables|SetIndexOffset 0)
              (Utilities|FlowControl|Sequence
                (:then_0
                  (bind _realindex_7 (CallFunction|GetVertexRealIndex (LocalVariables|GetCurrentRow) (LocalVariables|GetCurrentVertexIndex) Rows)))
                (:then_1
                  (bind _realindex_8 (CallFunction|GetVertexRealIndex (LocalVariables|GetCurrentRow) (LocalVariables|GetNextVertexIndex) Rows)))
                (:then_2
                  (bind _realindex_9 (CallFunction|GetVertexRealIndex (LocalVariables|GetNextRow) (+ (LocalVariables|GetCurrentVertexIndex) (LocalVariables|GetIndexOffset)) Rows)))
                (:then_3
                  (Utilities|Array|AppendArray (LocalVariables|GetTriangles) (Utilities|Array|MakeArray _realindex_7 _realindex_8 _realindex_9))))))
          (:B
            (for _index_6 (range 0 (- (LocalVariables|GetUsedVerticesCount) 2))
              (bind _output_get_7 (LocalVariables|SetCurrentVertexIndex _index_6))
              (LocalVariables|SetNextVertexIndex (+ _output_get_7 1))
              (LocalVariables|SetIndexOffset 1)
              (Utilities|FlowControl|Sequence
                (:then_0
                  (bind _realindex_10 (CallFunction|GetVertexRealIndex (LocalVariables|GetCurrentRow) (LocalVariables|GetCurrentVertexIndex) Rows)))
                (:then_1
                  (bind _realindex_11 (CallFunction|GetVertexRealIndex (LocalVariables|GetCurrentRow) (LocalVariables|GetNextVertexIndex) Rows)))
                (:then_2
                  (bind _realindex_12 (CallFunction|GetVertexRealIndex (LocalVariables|GetNextRow) (+ (LocalVariables|GetCurrentVertexIndex) (LocalVariables|GetIndexOffset)) Rows)))
                (:then_3
                  (Utilities|Array|AppendArray (LocalVariables|GetTriangles) (Utilities|Array|MakeArray _realindex_10 _realindex_11 _realindex_12)))))))))
    (:then_3
      (return (LocalVariables|GetTriangles)))))

(fn CreateVertexColors
  (params (VertexCount :type Integer))
  (for _index (range 0 VertexCount)
    (Utilities|Array|Add (LocalVariables|GetVertexColors) "(R=1.000000,G=1.000000,B=1.000000,A=1.000000)"))
  (return (LocalVariables|GetVertexColors)))

(fn CreateUV
  (params (VerticesCount :type Integer))
  (Math|Integer|CompareInt (Math|Integer|%(Integer) (- VerticesCount 1) 4)
    (:>
      (Utilities|Array|AppendArray (LocalVariables|GetUV) (Utilities|Array|MakeArray "(X=0.000000,Y=0.000000)"))
      (return (LocalVariables|GetUV)))
    (:==
      (for _index (range 0 (/ VerticesCount 3))
        (Utilities|Array|AppendArray (LocalVariables|GetUV) (Utilities|Array|MakeArray "(X=0.000000,Y=0.000000)" "(X=1.000000,Y=0.000000)" "(X=0.000000,Y=1.000000)")))
      (return (LocalVariables|GetUV)))))

(fn CreateTangets)

(fn GetRowVertexCount
  (params (RowNumber :type Integer) (Rows :type Integer))
  (Math|Integer|CompareInt (Math|Integer|%(Integer) RowNumber 2)
    (:>
      (return (- Rows 1)))
    (:==
      (return Rows))))

(fn GetRowsRangeVertexCount
  (params (LastRow :type Integer) (Rows :type Integer))
  (for _index (range 0 LastRow)
    (bind _vertexcount (CallFunction|GetRowVertexCount _index Rows))
    (LocalVariables|SetVertexCountSum (+ _vertexcount (LocalVariables|GetVertexCountSum))))
  (return (LocalVariables|GetVertexCountSum)))

(fn GetVertexRealIndex
  (params (Row :type Integer) (IndexInRow :type Integer) (Rows :type Integer))
  (bind _vertexcount (CallFunction|GetRowsRangeVertexCount (- Row 1) Rows))
  (return (+ _vertexcount IndexInRow)))